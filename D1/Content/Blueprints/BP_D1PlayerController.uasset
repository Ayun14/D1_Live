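; BP_D1PlayerController is a player controller that lets the player switch control between the pawns in the level.
; BeginPlay caches every Pawn actor into a Players array.
; Pressing 1 calls ChangePlayer with the current Index, then advances the Index, wrapping around by the array length.
; ChangePlayer unpossesses the current pawn and possesses the one at that index if it is valid.
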(event EventBeginPlay
  (bind _outactors (Actor|GetAllActorsOfClass "/Script/Engine.Pawn"))
  (Variables|Default|SetPlayers _outactors))

(event EventTick
  (params (DeltaSeconds :type Float%20%28single-precision%29)))

(event Input|KeyboardEvents|1
  (params (Key :type Key%20Structure :default "None"))
  (:Pressed
    (CallFunction|ChangePlayer (Variables|Default|GetIndex))
    (bind _result (Math|Integer|IncrementInt (Variables|Default|GetIndex))
      (:%20%20
        (Variables|Default|SetIndex (Math|Integer|%(Integer) _result (Utilities|Array|Length (Variables|Default|GetPlayers))))))))

(fn ConstructionScript)

(fn ChangePlayer
  (params (Index :type Integer))
  (Pawn|UnPossess)
  (if (Utilities|Array|IsValidIndex (Variables|Default|GetPlayers) Index)
    (Pawn|Possess (Utilities|Array|Get(acopy) (Variables|Default|GetPlayers) Index))))